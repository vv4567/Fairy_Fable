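; Fake 2D light actor that draws a procedural triangle-fan mesh with a light-source material, with a sphere sized to the light distance.
; Tick runs visibility traces per polygon side and builds fan indices, but trace rotation and vertex appending are disconnected and traces have zero length.
; CreatedMesh is only ever set false after section creation.
; A delayed check detects LightColor changes and pushes them to the dynamic material.
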(event `self.ReceiveBeginPlay`
  (set `self.LineTraceAngle` (/ 360.0 (`KismetMathLibrary.Conv_IntToDouble` (`self.Polygon`))))
  (set `self.OriginaColor` (`self.LightColor`)))

(event `self.ReceiveTick`
  (params (DeltaSeconds :type "Float (single-precision)"))
  (bind _returnvalue (`self.K2_GetActorLocation`))
  (bind _vertices_0 (`self.Vertices_0`))
  (`|ExecutionSequence`
    (:`then_0`
      (`KismetArrayLibrary.Array_Clear` (`self.UV0`))
      (`KismetArrayLibrary.Array_Clear` (`self.Triangles`))
      (`KismetArrayLibrary.Array_Clear` _vertices_0)
      (`KismetArrayLibrary.Array_Add` _vertices_0)
      (`KismetArrayLibrary.Array_Add` (`self.UV0`))
      (set `self.End` (`KismetMathLibrary.MakeVector` (`self.LightDIstance`)))
      (for _ (range (+ (`self.Polygon`) 1))
        (bind (_outhit _returnvalue_2) (`KismetSystemLibrary.LineTraceSingle` _returnvalue (+ _returnvalue (0.0 0.0 0.0)) "TraceTypeQuery1"))
        (set `self.bLineTRaceReturn` _returnvalue_2)
        (set `self.LineTRaceLocation` (- (`.Location` (`GameplayStatics.BreakHitResult` _outhit)) (`self.K2_GetActorLocation`))))
      (set `self.TriangleOffset` 1)
      (for _ (range (+ (- (`KismetArrayLibrary.Array_Length` (`self.Vertices`)) 3) 1))
        (`KismetArrayLibrary.Array_Add` (`self.Triangles`))
        (for _index (range 2)
          (`KismetArrayLibrary.Array_Add` (`self.Triangles`) (+ _index (`self.TriangleOffset`))))
        (`/Engine/EditorBlueprintResources/StandardMacros.IncrementInt` (`self.TriangleOffset`)))
      (if (`self.bCreatedMesh`)
        (`ProceduralMeshComponent.UpdateMeshSection_LinearColor` :`self` (`self.ProceduralMesh`) :`Vertices` (`self.Vertices_0`) :`UV0` (`self.UV0_0`))
        (else
          (`ProceduralMeshComponent.CreateMeshSection_LinearColor` :`self` (`self.ProceduralMesh`) :`Vertices` (`self.Vertices`) :`Triangles` (`self.Triangles`) :`UV0` (`self.UV0`))
          (`PrimitiveComponent.SetMaterial` (`self.ProceduralMesh`) 0 "/Game/Art/FakeLighting/M_LightSource.M_LightSource")
          (bind _returnvalue_3 (`PrimitiveComponent.CreateDynamicMaterialInstance` (`self.ProceduralMesh`) 0 "/Game/Art/FakeLighting/M_LightSource.M_LightSource" "None"))
          (`MaterialInstanceDynamic.SetVectorParameterValue` _returnvalue_3 "LightColor" (`self.LightColor`) :!label _label)
          (set `self.bCreatedMesh` false))))
    (:`then_1`
      (`KismetSystemLibrary.Delay` 0.2)
      (if (not (== (`self.LightColor`) (`self.OriginaColor`)))
        (`self.UPdatedCOlor`)
        (set `self.OriginaColor` (`self.LightColor`))))))

(event `UPdatedCOlor`
  (goto _label))

(fn `UserConstructionScript`
  (`SphereComponent.SetSphereRadius` (`self.Lightsphere`) (`self.LightDIstance`) true))