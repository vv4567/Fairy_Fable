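; Player controller for a 2D side-scroller that runs the player death and restart sequence.
; OnDeath destroys the player character, unpossesses it, fades the camera out and holds the fade while a death widget is shown.
; After a short delay it removes the widget and asks the 2DSideScrollerGameMode to restart the game.
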(event `OnDeath`
  (`self.K2_DestroyActor` (`GameplayStatics.GetPlayerCharacter` 0))
  (`self.UnPossess`)
  (`PlayerCameraManager.StartCameraFade` :`self` (`self.PlayerCameraManager`) :`ToAlpha` 1.0 :`Duration` 1.0 :`bHoldWhenFinished` true)
  (bind _returnvalue (`|CreateWidget` "/Game/Character/Blueprints/PlayerRelatedClasses/DeathWidget.DeathWidget_C" self))
  (`UserWidget.AddToViewport` _returnvalue 0)
  (`KismetSystemLibrary.Delay` 5.0)
  (`Widget.RemoveFromParent` _returnvalue)
  (bind _as2dside_scroller_game_mode (cast `/Game/Character/Blueprints/PlayerRelatedClasses/2DSideScrollerGameMode` (`GameplayStatics.GetGameMode`)))
  (`GameMode.RestartGame` _as2dside_scroller_game_mode))

(fn `UserConstructionScript`)